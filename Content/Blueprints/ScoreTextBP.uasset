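; ScoreTextBP is a score display that shows a running total on a TextRender and flashes it when points are added.
; Construction creates a dynamic material instance for the text.
; AddScore updates the total and text, then calls the BlinkText event, as functions cannot hold timelines, where a Timeline animates Emissive Power.
; A color blink is left disconnected, noted as failing to return to the original color.
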(event Custom|BlinkText
  (bind (_direction _emissive_power _color_change) (Timeline|Timeline_0 Play) ; Timeline qui update l'emissive du text
    (:Update
      (Rendering|Material|SetScalarParameterValue (Variables|Default|GetDynamicMat) "Emissive Power" _emissive_power :!class /Script/Engine.MaterialInstanceDynamic) ; Update du material du text
    )))

(fn ConstructionScript
  (bind _returnvalue (Rendering|Material|CreateDynamicMaterialInstance (Variables|Default|GetTextRender) 0 "/Game/Materials/M_TextMat_Inst.M_TextMat_Inst" "None" :!class /Script/Engine.PrimitiveComponent))
  (bind _output_get (Variables|Default|SetDynamicMat _returnvalue))
  (Rendering|Material|SetMaterial (Variables|Default|GetTextRender) 0 _output_get))

(fn AddScore
  (params (ScoreToAdd :type Float%20%28single-precision%29))
  (bind _output_get (Variables|Default|SetCurrentScore (+ ScoreToAdd (Variables|Default|GetCurrentScore))))
  (Rendering|Components|TextRender|SetText (Variables|Default|GetTextRender) (Utilities|Text|ToText(Float) _output_get "HalfToEven")) ; Set le text
  (CallFunction|BlinkText) ; Obligé de lancer ce custom event car il est impossible d'avoir une timeline dans une fonction
)