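; TimerText is a stopwatch that displays elapsed minutes and seconds on two separate text elements.
; While the TimerPlay flag is set, Tick accumulates delta time and writes the seconds with two-digit padding and up to two decimals.
; Passing 60 seconds increments the minutes text and zeroes the seconds, discarding any overshoot.
; TimerStart and TimerStop only toggle the flag, so restarting resumes from the current time.
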(event EventTick
  (params (DeltaSeconds :type Float%20%28single-precision%29))
  (if (Variables|Default|GetTimerPlay)
    (Variables|Default|Setseconds (+ (Variables|Default|Getseconds) DeltaSeconds))
    (Rendering|Components|TextRender|SetText (Variables|Default|GetTextSeconds) (Utilities|Text|ToText(Float) (Variables|Default|Getseconds) "HalfToEven" false true 2 324 0 2))
    (if (> (Variables|Default|Getseconds) 6e+01)
      (Variables|Default|Setminutes (+ (Variables|Default|Getminutes) 1.0))
      (Variables|Default|Setseconds 0.0)
      (Rendering|Components|TextRender|SetText (Variables|Default|GetTextMinutes) (Utilities|Text|ToText(Float) (Variables|Default|Getminutes) "HalfToEven")))))

(fn ConstructionScript)

(fn TimerStart
  (Variables|Default|SetTimerPlay true))

(fn TimerStop
  (Variables|Default|SetTimerPlay false))