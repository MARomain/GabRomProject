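; Hover component that pushes its owner away from the ground using physics forces.
; On BeginPlay it enables physics simulation on the owner's first primitive component.
; Each Tick it traces straight down from its own location over TraceLenght, with debug drawing.
; On a hit it prints a debug string and applies force along the impact normal to follow slopes, fading linearly from strongest up close to zero at full trace length.
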(event EventBeginPlay
  (bind _output_get (Variables|Default|SetPrimitive%20Component (Utilities|Array|Get(acopy) (Actor|GetComponentsByClass (Components|GetOwner) "/Script/Engine.PrimitiveComponent"))))
  (Physics|SetSimulatePhysics _output_get true))

(event EventTick
  (params (DeltaSeconds :type Float%20%28single-precision%29))
  (bind _returnvalue (Transformation|GetWorldLocation))
  (bind (_outhit _returnvalue_2) (Collision|LineTraceByChannel _returnvalue (- _returnvalue (Math|Vector|MakeVector 0.0 0.0 (Variables|Default|GetTrace%20Lenght))) "TraceTypeQuery1" false 0 "ForDuration")) ; LineTrace de l'objet à Z - TraceLenght
  (if _returnvalue_2 ; SI ça hit quelques chose
    (Development|PrintString "Hello")
    (Physics|AddForce (Variables|Default|GetPrimitive%20Component) (* (.impactnormal _outhit) (Math|Float|Lerp 1e+04 0.0 (/ (Math|Vector|VectorLength (- (.location _outhit) (Transformation|GetWorldLocation))) (Variables|Default|GetTrace%20Lenght)))) "None" false)))