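; Interactive door Blueprint that slides between an open and a closed position when interacted with.
; Each Interact event flips InteractState and plays or reverses DoorTimeline, whose interpolation track lerps the Door's relative location between StartLocation and EndLocation.
; GetInteractState exposes the current toggle state, while LevelComm and the construction script are empty.
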(event EventInteract
  (if (Variables|Default|GetInteractState)
    (Variables|Default|SetInteractState false)
    (bind _doorinterpolation (Timeline|DoorTimeline Reverse)
      (:Update
        (Transformation|SetRelativeLocation (Variables|Default|GetDoor) (Math|Vector|Lerp(Vector) (Variables|Default|GetStartLocation) (Variables|Default|GetEndLocation) _doorinterpolation) false false)))
    (else
      (Variables|Default|SetInteractState true)
      (Timeline|DoorTimeline Play))))

(fn ConstructionScript)

(fn GetInteractState
  (return (Variables|Default|GetInteractState)))

(fn LevelComm)