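; ShootToEnd is a shootable actor that stops the timer and slides its mesh to a new position when shot.
; Its construction script gives the mesh a dynamic glow material.
; If not already flagged as hit, InteractwithShoot calls TimerStop through the TimerText actors, recolors the mesh, switches the text to green, then moves the mesh by timed interpolation after a delay.
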(event EventInteractwithShoot
  (if (not (Variables|Default|GetHasBeenHit))
    ;[1 1 1] Stop le timer
    (bind _astimer_text (Utilities|Casting|CastToTimerTextClass "/Game/Blueprints/TimerText.TimerText_C"))
    (bind _outactors (Actor|GetAllActorsOfClass _astimer_text))
    (Default|TimerStop _outactors)
    ;[1 1 1] Update graphics
    (Rendering|Material|SetVectorParameterValueonMaterials (Variables|Default|GetMesh) "color" (Math|Conversions|ToVector(LinearColor) (Variables|Default|GetcolorWhenHit)))
    (Rendering|Material|SetMaterial (Variables|Default|GetText) 0 "/Game/Materials/M_TextMat_Inst_Green.M_TextMat_Inst_Green")
    ;[1 1 1] Move Object
    (Utilities|FlowControl|Delay (Variables|Default|GetDelayBeforeOpening))
    (Components|MoveComponentTo (Variables|Default|GetMesh) (Variables|Default|GetMoveRelativeLocation) "0, 0, 0" false false (Variables|Default|GetTimeToMove) false)))

(fn ConstructionScript
  (bind _returnvalue (Rendering|Material|CreateDynamicMaterialInstance "/Game/Materials/GlowEnhanced_Inst.GlowEnhanced_Inst" "None" :!class /Script/Engine.KismetMaterialLibrary))
  (bind _output_get (Variables|Default|SetdynamicMat _returnvalue))
  (Rendering|Material|SetMaterial (Variables|Default|GetMesh) 0 _output_get))