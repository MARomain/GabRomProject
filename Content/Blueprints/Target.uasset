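; Shootable target actor that loses health through its DoDamage event and awards score when destroyed.
; The construction script sets starting health, light intensity and a dynamic glow material on the cube.
; Non-lethal hits play a timeline that animates glow and light intensity.
; On death, a DoOnce recolors material and light, then finds actors by class to add score and decrement the ShootToEnd and TargetCounterText target counts.
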(event EventDoDamage
  (params (Damage :type Float%20%28single-precision%29))
  ;[1 1 1] Update Health
  (Variables|Default|SetcurrentHealth (- (Variables|Default|GetcurrentHealth) Damage)) ; On diminue la vie de la target
  (if (<= (Variables|Default|GetcurrentHealth) 0.0) ; Si la cible est dead
    (Utilities|FlowControl|DoOnce false
      (:Completed
        ;[1 1 1] Update Graphics
        (Rendering|Material|SetVectorParameterValue (Variables|Default|GetdynamicMat) "color" (Variables|Default|GetDeadColor) :!class /Script/Engine.MaterialInstanceDynamic) ; On change sa couleur
        (Rendering|Components|Light|SetLightColor (Variables|Default|GetPointLight) (Variables|Default|GetDeadColor) true) ; Et la couleur de la light
        ;[1 1 1] Update score
        (bind _asscore_text_bp (Utilities|Casting|CastToScoreTextBPClass "/Game/Blueprints/ScoreTextBP.ScoreTextBP_C")) ; On envoie à tout les ScoreTextBP (score 3D)
        ;;[1 1 1] Avoir une référence avec un array de score en publique et référencé tout dans le details pannel peut être ?
        ;; Ou en tout cas prendre la référence une fois au début et la stocké par la chopper à chaque fois que je kill une target
        (bind _outactors (Actor|GetAllActorsOfClass _asscore_text_bp)) ; Recupère les acteurs de cette classe
        (Default|AddScore _outactors (Variables|Default|GettargetScore)) ; Fonction dans Le BP Score
        (bind _outactors_2 (Actor|GetAllActorsOfClass "/Game/Blueprints/ShootToEnd.ShootToEnd_C"))
        (Variables|/Game/Blueprints/ShootToEnd.ShootToEnd_C|SettargetsLeft (Utilities|Array|Get(acopy) _outactors_2) (- (Variables|/Game/Blueprints/ShootToEnd.ShootToEnd_C|GettargetsLeft (Utilities|Array|Get(acopy) _outactors_2)) 1))
        (bind _outactors_3 (Actor|GetAllActorsOfClass "/Game/Blueprints/TargetCounterText.TargetCounterText_C"))
        (bind _output_get (Variables|/Game/Blueprints/TargetCounterText.TargetCounterText_C|SettargetAlive (Utilities|Array|Get(acopy) _outactors_3) (- (Variables|/Game/Blueprints/TargetCounterText.TargetCounterText_C|GettargetAlive (Utilities|Array|Get(acopy) _outactors_3)) 1)))
        (Rendering|Components|TextRender|SetText (Variables|/Game/Blueprints/TargetCounterText.TargetCounterText_C|GetTextTargetAlive (Utilities|Array|Get(acopy) _outactors_3)) (Utilities|Text|ToText(Integer) _output_get))))
    (else
      ;[1 1 1] Update graphics
      (bind (_direction _emissive_strenght _light_strenght) (Timeline|LightBlink PlayFromStart) ; Utilisations d'une timeline pour faire varier l'intensité de la light / glow
        (:Update
          (Rendering|Material|SetScalarParameterValue (Variables|Default|GetdynamicMat) "Glow Strenght" _emissive_strenght :!class /Script/Engine.MaterialInstanceDynamic) ; Update du glow
          (Rendering|Components|Light|SetIntensity (Variables|Default|GetPointLight) _light_strenght) ; Update de la light
        )))))

(fn ConstructionScript
  (Variables|Default|SetcurrentHealth (Variables|Default|GetstartingHealth))
  (bind _returnvalue (Rendering|Material|CreateDynamicMaterialInstance "/Game/Materials/GlowEnhanced_Inst.GlowEnhanced_Inst" "None" :!class /Script/Engine.KismetMaterialLibrary))
  (bind _output_get (Variables|Default|SetdynamicMat _returnvalue))
  (Rendering|Material|SetMaterial (Variables|Default|GetCube) 0 _output_get)
  (Rendering|Components|Light|SetIntensity (Variables|Default|GetPointLight) (Variables|Default|GetlightIntensity)))