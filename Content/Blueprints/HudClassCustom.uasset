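; HUD class that draws a centered first-person crosshair and puts the ammo widget on screen.
; BeginPlay caches the player controller and Controller_Unreal_Neon character, then creates the AmmoCount widget and passes CurrentAmmo to CallUpdateAmmoUI.
; DrawHUD draws the crosshair texture at screen center, sized by CrossHairSize.
; A matching HealthUI setup function exists, but its call is disconnected, so the health widget is not created here.
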(event EventBeginPlay
  (CallFunction|GetReferences)
  (CallFunction|CreateAmmoHUD))

(event EventDrawHUD
  (params (SizeX :type Integer) (SizeY :type Integer))
  (CallFunction|CreateCrosshair SizeX SizeY))

(fn ConstructionScript)

(fn CreateCrosshair
  (params (A :type Integer) (A2 :type Integer))
  (bind _crosshairsize (Variables|Default|GetcrossHairSize))
  (bind _returnvalue (/ _crosshairsize 2.0))
  (Canvas|DrawTexture "/Game/FirstPerson/Textures/FirstPersonCrosshair.FirstPersonCrosshair" (- (Math|Conversions|ToFloat(Integer) (/ A 2)) _returnvalue) (- (Math|Conversions|ToFloat(Integer) (/ A2 2)) _returnvalue) _crosshairsize _crosshairsize 0.0 0.0 1.0 1.0 (Utilities|Struct|MakeLinearColor 1.0 1.0 1.0 1.0)))

(fn CreateHealthHUD
  (bind _returnvalue (UserInterface|CreateWidget "/Game/Blueprints/HealthUI.HealthUI_C" (Variables|Default|GetPlayerControllerReference)))
  (UserInterface|Viewport|AddtoViewport _returnvalue 0)
  (Default|CallUpdateHealthUI (Variables|/Game/Blueprints/Controller_Unreal_Neon.Controller_Unreal_Neon_C|GetHealth (Variables|Default|GetUnrealNeonControllerReference))))

(fn CreateAmmoHUD
  (bind _returnvalue (UserInterface|CreateWidget "/Game/Blueprints/AmmoCount.AmmoCount_C" (Variables|Default|GetPlayerControllerReference)))
  (UserInterface|Viewport|AddtoViewport _returnvalue 0)
  (Default|CallUpdateAmmoUI (Variables|/Game/Blueprints/Controller_Unreal_Neon.Controller_Unreal_Neon_C|GetCurrentAmmo (Variables|Default|GetUnrealNeonControllerReference))))

(fn GetReferences
  (Variables|Default|SetPlayerControllerReference (Game|GetPlayerController 0))
  (Variables|Default|SetUnrealNeonControllerReference (.AsController%20Unreal%20Neon (Utilities|Casting|CastToController_Unreal_Neon (Game|GetPlayerCharacter 0)))))