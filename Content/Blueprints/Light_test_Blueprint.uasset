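; Light test Blueprint actor that switches a point light on while something overlaps its trigger volume.
; Trigger begin and end overlap events show and hide the PointLight, with no filter on the overlapping actor.
; The construction script applies the LightToggle, LightIntensity and LightColor variables to set the light's initial visibility, brightness and color.
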(event OnComponentBeginOverlap(Trigger)
  (params (OverlappedComponent :type Primitive%20Component%20Object%20Reference) (OtherActor :type Actor%20Object%20Reference) (OtherComp :type Primitive%20Component%20Object%20Reference) (OtherBodyIndex :type Integer) (bFromSweep :type Boolean) (SweepResult :type Hit%20Result%20Structure%20%28by%20ref%29))
  (Rendering|SetVisibility (Variables|Default|GetPointLight) true false))

(event OnComponentEndOverlap(Trigger)
  (params (OverlappedComponent :type Primitive%20Component%20Object%20Reference) (OtherActor :type Actor%20Object%20Reference) (OtherComp :type Primitive%20Component%20Object%20Reference) (OtherBodyIndex :type Integer))
  (Rendering|SetVisibility (Variables|Default|GetPointLight) false false))

(fn ConstructionScript
  (bind _pointlight (Variables|Default|GetPointLight))
  (Rendering|SetVisibility _pointlight (Variables|Default|GetlightToggle) false)
  (Rendering|Components|Light|SetIntensity _pointlight (Variables|Default|GetlightIntensity))
  (Rendering|Components|Light|SetLightColor _pointlight (Variables|Default|GetlightColor) true))