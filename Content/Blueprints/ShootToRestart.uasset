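; A shootable restart target that reloads the current level when hit.
; On InteractwithShoot it recolors the cube through its "color" material parameter and switches the text to a green material as hit feedback.
; After a configurable delay, it looks up the current level name and reopens that level.
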(event EventInteractwithShoot
  (Rendering|Material|SetVectorParameterValueonMaterials (Variables|Default|GetCube) "color" (Math|Conversions|ToVector(LinearColor) (Variables|Default|GetcolorWhenHit)))
  (Rendering|Material|SetMaterial (Variables|Default|Gettext) 0 "/Game/Materials/M_TextMat_Inst_Green.M_TextMat_Inst_Green")
  (Utilities|FlowControl|Delay (Variables|Default|GetdelayBeforeRestart))
  (bind _returnvalue (Game|GetCurrentLevelName true))
  (Game|OpenLevel(byName) (Utilities|String|StringToName _returnvalue)))

(fn ConstructionScript)