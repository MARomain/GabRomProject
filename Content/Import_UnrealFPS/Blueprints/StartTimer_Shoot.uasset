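; StartTimer_Shoot is a door that turns green and moves up when its StartTimerAnimation flag is set, which a comment attributes to FirstPersonCharacter.
; Tick polls the flag as a workaround for non-working hit events, sets the Cube's emissive color, waits briefly, then moves it to MoveUpDistance in relative Z.
; The flag is never reset here, the overlap event is empty, and leftover code setting the controller's StartTimer is unconnected.
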(event OnComponentBeginOverlap(Collider)
  (params (OverlappedComponent :type Primitive%20Component%20Object%20Reference) (OtherActor :type Actor%20Object%20Reference) (OtherComp :type Primitive%20Component%20Object%20Reference) (OtherBodyIndex :type Integer) (bFromSweep :type Boolean) (SweepResult :type Hit%20Result%20Structure%20%28by%20ref%29))
  ;[1 1 1] Old way, quand on passe dans le trigger (avec overlapall dans le collider)
)

(event EventTick
  (params (DeltaSeconds :type Float%20%28single-precision%29))
  ;[1 1 1] J'arrive pas à trouver pourquoi je peux pas détecter la collision avec un "event hit" du coup le FirstPersonCharacter me passe une varible que je check à chaque frame
  (if (Variables|Default|GetStartTimerAnimation)
    (Rendering|Material|SetVectorParameterValueonMaterials (Variables|Default|GetCube) "Emissive color" (Math|Conversions|ToVector(LinearColor) "(R=0.016807,G=0.921582,B=0.198069,A=1.000000)")) ; On change la couleur de la porte
    (Utilities|FlowControl|Delay 0.5) ; On attend un peu
    (Components|MoveComponentTo (Variables|Default|GetCube) (Math|Vector|MakeVector 0.0 0.0 (Variables|Default|GetMoveUpDistance)) (Variables|/Script/Engine.SceneComponent|GetRelativeRotation (Variables|Default|GetCube)) false false 1.0 false) ; RELATIVE TO THE ROOT COMPONENT (check actual component position from the root first)
  ))

(fn ConstructionScript)