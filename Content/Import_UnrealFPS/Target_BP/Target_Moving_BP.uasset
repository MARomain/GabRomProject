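; Moving shooting target that takes damage from hits and awards score to the hitter once its health runs out.
; A Tick-driven timeline lerps it between two endpoints, computed at BeginPlay as offsets from its starting location.
; Non-lethal hits play a timeline pulsing the dynamic material glow and point light intensity.
; The lethal hit, gated by DoOnce, sends the score and turns both material and light green, leaving the target in place.
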(event EventHandleHit
  (params (Hitter :type Actor%20Object%20Reference) (Damage :type Integer))
  (Variables|Default|SetHitter Hitter)
  (Variables|Default|SetDamageValue Damage)
  (Variables|Default|SetCurrentHealth (- (Variables|Default|GetCurrentHealth) (Variables|Default|GetDamageValue)))
  (if (<= (Variables|Default|GetCurrentHealth) 0)
    (Utilities|FlowControl|DoOnce false
      (:Completed
        (Class|CharacterBPI|HandleUpdateScore(Message) (Variables|Default|GetHitter) (Variables|Default|GetTargetScore))
        (Rendering|Material|SetVectorParameterValue (Variables|Default|GetDynamicMat) "color" "(R=0.016807,G=0.921582,B=0.198069,A=1.000000)" :!class /Script/Engine.MaterialInstanceDynamic)
        (Rendering|Components|Light|SetLightColor (Variables|Default|GetPointLight) "(R=0.016807,G=0.921582,B=0.198069,A=1.000000)" true)))
    (else
      (bind (_direction _glow_strenght _light_strenght) (Timeline|Timeline_2 PlayFromStart)
        (:Update
          (Rendering|Material|SetScalarParameterValue (Variables|Default|GetDynamicMat) "Glow Strenght" _glow_strenght :!class /Script/Engine.MaterialInstanceDynamic)
          (Rendering|Components|Light|SetIntensity (Variables|Default|GetPointLight) (* _light_strenght (Variables|Default|GetLight%20intensity))))))))

(event EventBeginPlay
  (bind _returnvalue (Transformation|GetActorLocation))
  (bind _output_get (Variables|Default|SetPos1 (+ _returnvalue (Variables|Default|GetStartLocation%20))))
  (bind _output_get_2 (Variables|Default|SetPos2 (+ _returnvalue (Variables|Default|GetEndLocation))))
  (Variables|Default|SetCurrentHealth (Variables|Default|GetStarting%20health))
  (bind _returnvalue_2 (Rendering|Material|CreateDynamicMaterialInstance "/Game/Materials/GlowEnhanced_Inst.GlowEnhanced_Inst" "None" :!class /Script/Engine.KismetMaterialLibrary))
  (Variables|Default|SetDynamicMat _returnvalue_2)
  (Rendering|Material|SetMaterial (Variables|Default|GetCube) 0 (Variables|Default|GetDynamicMat))
  (Rendering|Components|Light|SetIntensity (Variables|Default|GetPointLight) (Variables|Default|GetLight%20intensity)))

(event EventTick
  (params (DeltaSeconds :type Float%20%28single-precision%29))
  (bind _track (Timeline|Timeline_3 Play)
    (:Update
      (Transformation|SetActorRelativeLocation (Math|Vector|Lerp(Vector) (stale EventBeginPlay _output_get) (stale EventBeginPlay _output_get_2) _track)))))

(fn ConstructionScript)